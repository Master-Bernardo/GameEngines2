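; Enemy Blueprint with health that takes damage and can turn to face a character.
; The AnyDamage event feeds RecieveDamage, which subtracts from Health, prints the remaining value, and destroys the actor at zero or below.
; LookAtPlayer snaps the actor's full rotation toward a given character's location using FindLookAtRotation, but nothing in this Blueprint calls it.
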(event Game|Damage|EventAnyDamage
  (params (Damage :type Float%20%28single-precision%29) (DamageType :type Damage%20Type%20Object%20Reference) (InstigatedBy :type Controller%20Object%20Reference) (DamageCauser :type Actor%20Object%20Reference))
  (CallFunction|RecieveDamage Damage))

(fn ConstructionScript)

(fn RecieveDamage
  (params (Damage :type Float%20%28single-precision%29))
  (Variables|Default|Sethealth (- (Variables|Default|Gethealth) Damage))
  (if (<= (Variables|Default|Gethealth) 0.0)
    (Development|PrintString "Dieded")
    (Actor|DestroyActor)
    (else
      (Development|PrintString (Utilities|String|Append "Health: " (Utilities|String|ToString(Float) (Variables|Default|Gethealth)))))))

(fn LookatPlayer
  (params (CharacterToLookAt :type Actor%20Object%20Reference))
  ;[1 1 1] Look At Athe Player
  (Transformation|SetActorRotation (Math|Rotator|FindLookatRotation (Transformation|GetActorLocation) (Transformation|GetActorLocation CharacterToLookAt))))