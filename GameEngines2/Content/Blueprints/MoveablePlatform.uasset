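; A moving platform actor that shuttles back and forth between the locations of two referenced actors, To and From, starting toward To.
; Tick moves it toward CurrentTarget at MovementSpeed, scaled by delta time, without sweep.
; Once within a small tolerance of the target, a Delay precedes flipping MovingBack and switching targets.
; Movement is not paused during that Delay, so the platform keeps stepping around the endpoint.
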(event EventTick
  (params (DeltaSeconds :type Float%20%28single-precision%29))
  (bind _self self)
  (bind _returnvalue (Transformation|GetActorLocation _self))
  (Transformation|SetActorLocation (+ _returnvalue (* (Math|Vector|GetUnitDirection(Vector) _returnvalue (Variables|Default|GetCurrentTarget)) (* (Variables|Default|GetMovementSpeed) DeltaSeconds))) false false)
  (if (Math|Vector|Equal(Vector) (Transformation|GetActorLocation self) (Variables|Default|GetCurrentTarget) 5.0)
    (Utilities|FlowControl|Delay 2.0)
    (if (Variables|Default|GetMovingBack)
      (Variables|Default|SetCurrentTarget (Transformation|GetActorLocation (Variables|Default|GetTo)))
      (Variables|Default|SetMovingBack false)
      (else
        (Variables|Default|SetCurrentTarget (Transformation|GetActorLocation (Variables|Default|GetFrom)))
        (Variables|Default|SetMovingBack true)))))

(event EventBeginPlay
  (Variables|Default|SetCurrentTarget (Transformation|GetActorLocation (Variables|Default|GetTo))))

(fn ConstructionScript)