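; EnemyTurrent is an enemy turret that turns to face the player and fires projectiles when it sees them.
; Its PawnSensing OnSeePawn event casts to FirstPersonCharacter, then snaps the whole actor's rotation toward that character.
; It spawns a FirstPersonProjectile at ProjectileSpawnLocation and launches it with a forward impulse scaled by ShootForce.
; A SpawnProjectile flag and a TimeBetweenShots delay throttle the fire rate.
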(event OnSeePawn(PawnSensing)
  (params (Pawn :type Pawn%20Object%20Reference))
  (bind _asfirst_person_character (Utilities|Casting|CastToFirstPersonCharacter Pawn))
  (Utilities|FlowControl|Sequence
    (:then_0
      ;[1 1 1] Look At Athe Player
      (Transformation|SetActorRotation (Math|Rotator|FindLookatRotation (Transformation|GetActorLocation) (Transformation|GetActorLocation _asfirst_person_character))))
    (:then_1
      ;[1 1 1] Shoot
      (if (Variables|Default|GetspawnProjectile)
        (bind _returnvalue (Game|SpawnActorfromClass "/Game/Blueprints/FirstPersonBP/Blueprints/FirstPersonProjectile.FirstPersonProjectile_C" (Transformation|GetWorldTransform (Variables|Default|GetProjectileSpawnLocation)) "Undefined" 0 0))
        (Physics|AddImpulse (Variables|/Game/Blueprints/FirstPersonBP/Blueprints/FirstPersonProjectile.FirstPersonProjectile_C|GetSphere _returnvalue) (* (Math|Vector|GetForwardVector (Variables|Default|GetProjectileSpawnLocation)) (Variables|Default|GetshootForce)) "None" false)
        (Variables|Default|SetspawnProjectile false)
        (Utilities|FlowControl|Delay (Variables|Default|GettimeBetweenShots))
        (Variables|Default|SetspawnProjectile true)))))

(fn ConstructionScript)