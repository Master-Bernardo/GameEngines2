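; Enemy turret actor that turns toward the player and fires projectiles when its PawnSensing component sees a FirstPersonCharacter.
; Each sighting calls LookAtPlayer, then spawns a FirstPersonProjectile at the ProjectileSpawnLocation transform.
; The SpawnProjectile flag and a TimeBetweenShots delay throttle the fire rate.
; An AddImpulse node using ShootForce is left disconnected, as the projectile already has its own impulse.
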(event OnSeePawn(PawnSensing)
  (params (Pawn :type Pawn%20Object%20Reference))
  (bind _asfirst_person_character (Utilities|Casting|CastToFirstPersonCharacter Pawn))
  (Utilities|FlowControl|Sequence
    (:then_0
      (CallFunction|LookatPlayer _asfirst_person_character))
    (:then_1
      ;[1 1 1] Shoot
      (if (Variables|Default|GetspawnProjectile)
        (bind _returnvalue (Game|SpawnActorfromClass "/Game/Blueprints/FirstPersonBP/Blueprints/FirstPersonProjectile.FirstPersonProjectile_C" (Transformation|GetWorldTransform (Variables|Default|GetProjectileSpawnLocation)) "Undefined" 0 0))
        (Variables|Default|SetspawnProjectile false)
        (Utilities|FlowControl|Delay (Variables|Default|GettimeBetweenShots))
        (Variables|Default|SetspawnProjectile true)))))

(fn ConstructionScript
  (|CallParentFunction))